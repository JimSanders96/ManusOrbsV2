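; BP_LuggageSpawner is an actor that spawns and launches luggage orbs for a border control game.
; SpawnLuggage picks a class from LuggageTypes, with the random index capped at 1, and spawns it at SpawnPoint with sound and particles.
; It pushes the orb's collision along SpawnPoint's forward vector through the I_Orb interface, then registers it with BorderControlGameState.
; ClearLuggage destroys BP_OrbParent actors from an array.
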(event EventBeginPlay)

(event EventActorBeginOverlap
  (params (OtherActor :type Actor%20Object%20Reference)))

(event EventTick
  (params (DeltaSeconds :type Float%20%28single-precision%29)))

(fn ConstructionScript)

(fn SpawnLuggage
  (bind _spawnpoint (Variables|Default|GetSpawnPoint))
  (bind _luggagetypes (Variables|Default|GetLuggageTypes))
  (bind _returnvalue (Transformation|GetWorldLocation _spawnpoint))
  (bind _returnvalue_2 (Game|SpawnActorfromClass (Utilities|Array|Get(acopy) _luggagetypes (Math|Random|RandomIntegerinRange 0 (Math|Integer|Min(Integer) (Utilities|Array|Length _luggagetypes) 1))) (Transformation|GetWorldTransform (Variables|Default|GetSpawnPoint)) "Undefined" 0 0))
  (bind _asi_orb (Utilities|Casting|CastToI_Orb _returnvalue_2))
  (bind _collision (Default|GetCollision _asi_orb))
  (Audio|PlaySoundatLocation "/Game/FirstPerson/Audio/FirstPersonTemplateWeaponFire02.FirstPersonTemplateWeaponFire02" _returnvalue "0, 0, 0" 0.05 0.1)
  (Effects|SpawnEmitteratLocation "/Game/InfinityBladeEffects/Effects/FX_Ability/Defense/P_Shield_Spawn.P_Shield_Spawn" _returnvalue)
  (Physics|AddForce _collision (* (Math|Vector|GetForwardVector (Variables|Default|GetSpawnPoint)) (Variables|Default|GetSpawnForce)) "None" false)
  (bind _asborder_control_game_state (Utilities|Casting|CastToBorderControlGameState (Game|GetGameState)))
  (Default|AddLuggage _asborder_control_game_state _asi_orb))

(fn ClearLuggage
  (for _array_element 0
    (bind _asbp_orb_parent (Utilities|Casting|CastToBP_OrbParent _array_element))
    (Actor|DestroyActor _asbp_orb_parent)))