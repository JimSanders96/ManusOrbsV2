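; BP_LuggageReciever is a drop-off actor that registers orbs as received luggage in the border control game.
; It caches the BorderControlGameState on BeginPlay, printing an error if the cast fails.
; When an actor implementing I_Orb begins overlapping its Box, it passes that actor to the game state's RecievedLuggage and spawns the P_Shield_Spawn particle effect at RecievePoint.
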(event OnComponentBeginOverlap(Box)
  (params (OtherActor :type Actor%20Object%20Reference) (OtherComp :type Primitive%20Component%20Object%20Reference) (OtherBodyIndex :type Integer) (bFromSweep :type Boolean) (SweepResult :type Hit%20Result%20Structure%20%28by%20ref%29))
  (if (Utilities|DoesObjectImplementInterface OtherActor "/Game/Interfaces/I_Orb.I_Orb_C")
    (bind _asi_orb (Utilities|Casting|CastToI_Orb OtherActor))
    (Default|RecievedLuggage (Variables|Default|GetBorderPatrolGameState) _asi_orb)
    (Effects|SpawnEmitteratLocation "/Game/InfinityBladeEffects/Effects/FX_Ability/Defense/P_Shield_Spawn.P_Shield_Spawn" (Transformation|GetWorldLocation (Variables|Default|GetRecievePoint)))))

(event EventBeginPlay
  (bind _asborder_control_game_state (Utilities|Casting|CastToBorderControlGameState (Game|GetGameState))
    (:then
      (Variables|Default|SetBorderPatrolGameState _asborder_control_game_state))
    (:CastFailed
      (Development|PrintString "Cast failed"))))

(event EventTick
  (params (DeltaSeconds :type Float%20%28single-precision%29)))

(fn ConstructionScript)