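; Game state for a border control game that coordinates the luggage flow between a spawner and a receiver.
; The construction script caches the first luggage receiver and spawner found in the world.
; Spawning new luggage sends all tracked pieces to the receiver's receive point, then requests a fresh batch from the spawner.
; Luggage is registered through AddLuggage, then untracked and destroyed through RecievedLuggage.
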(event EventBeginPlay)

(event EventTick
  (params (DeltaSeconds :type Float%20%28single-precision%29)))

(fn ConstructionScript
  (bind _outactors (Actor|GetAllActorsOfClass "/Game/Blueprints/Actors/BP_LuggageReciever.BP_LuggageReciever_C"))
  (Variables|Default|SetReciever (Utilities|Array|Get(acopy) _outactors))
  (bind _outactors_2 (Actor|GetAllActorsOfClass "/Game/Blueprints/Actors/BP_LuggageSpawner.BP_LuggageSpawner_C"))
  (Variables|Default|SetSpawner (Utilities|Array|Get(acopy) _outactors_2)))

(fn AddLuggage
  (params (Luggage :type I%20Orb%20Interface))
  (Utilities|Array|Add (Variables|Default|GetTotalLuggage) Luggage))

(fn SpawnNewLuggage
  (for _array_element (Variables|Default|GetTotalLuggage)
    (bind _newparam (CallFunction|GetRecieverLocation))
    (Default|StartMoving _array_element _newparam true))
  (for _index (range 0 5)
    (Default|SpawnLuggage (Variables|Default|GetSpawner))))

(fn GetRecieverLocation
  (return (Transformation|GetWorldLocation (Variables|/Game/Blueprints/Actors/BP_LuggageReciever.BP_LuggageReciever_C|GetRecievePoint (Variables|Default|GetReciever)))))

(fn RecievedLuggage
  (params (Luggage :type I%20Orb%20Interface))
  (Utilities|Array|RemoveItem (Variables|Default|GetTotalLuggage) Luggage)
  (bind _asactor (Utilities|Casting|CastToActor Luggage))
  (Actor|DestroyActor _asactor))