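; VR pawn that collects elemental orbs with each hand and fires them, with gun components following the motion controllers every tick.
; While a trigger is held, overlapped orbs matching that hand's first orb type are queued.
; On release, the MultiFireLoop macro launches them one by one along controller forward, using force and a delay.
; Index functions swap Manus hand materials and element sounds; older glove-grab logic remains disconnected.
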(event OnComponentBeginOverlap(Left)
  (params (OverlappedComponent :type Primitive%20Component%20Object%20Reference) (OtherActor :type Actor%20Object%20Reference) (OtherComp :type Primitive%20Component%20Object%20Reference) (OtherBodyIndex :type Integer) (bFromSweep :type Boolean) (SweepResult :type Hit%20Result%20Structure%20%28by%20ref%29))
  (bind _orbsl (Variables|Default|GetOrbsL))
  (bind _item (Utilities|Array|Get(acopy) _orbsl))
  (if (Variables|Default|GetIsPressedL)
    (bind _asbp_orb_parent (Utilities|Casting|CastToBP_OrbParent OtherActor))
    (Utilities|IsValid _item
      (:Is%20Valid
        (Math|Integer|CompareInt (Variables|/Game/Orbs/BP_OrbParent.BP_OrbParent_C|GetOrbIndex _asbp_orb_parent) (Variables|/Game/Orbs/BP_OrbParent.BP_OrbParent_C|GetOrbIndex _item)
          (:==
            _)))
      (:Is%20Not%20Valid
        _))
    (Utilities|Array|Add (Variables|Default|GetOrbsL) _asbp_orb_parent)
    (Variables|/Game/Orbs/BP_OrbParent.BP_OrbParent_C|SetIsCollected _asbp_orb_parent true)
    (Effects|SpawnEmitteratLocation "/Game/InfinityBladeEffects/Effects/FX_Ability/Defense/P_Shield_Spawn.P_Shield_Spawn" (Transformation|GetActorLocation OtherActor))))

(event OnComponentBeginOverlap(Right)
  (params (OverlappedComponent :type Primitive%20Component%20Object%20Reference) (OtherActor :type Actor%20Object%20Reference) (OtherComp :type Primitive%20Component%20Object%20Reference) (OtherBodyIndex :type Integer) (bFromSweep :type Boolean) (SweepResult :type Hit%20Result%20Structure%20%28by%20ref%29))
  (bind _orbsr (Variables|Default|GetOrbsR))
  (bind _item (Utilities|Array|Get(acopy) _orbsr))
  (if (Variables|Default|GetIsPressedR)
    (bind _asbp_orb_parent (Utilities|Casting|CastToBP_OrbParent OtherActor))
    (Utilities|IsValid _item
      (:Is%20Valid
        (Math|Integer|CompareInt (Variables|/Game/Orbs/BP_OrbParent.BP_OrbParent_C|GetOrbIndex _item) (Variables|/Game/Orbs/BP_OrbParent.BP_OrbParent_C|GetOrbIndex _asbp_orb_parent)
          (:==
            _)))
      (:Is%20Not%20Valid
        _))
    (Utilities|Array|Add (Variables|Default|GetOrbsR) _asbp_orb_parent)
    (Variables|/Game/Orbs/BP_OrbParent.BP_OrbParent_C|SetIsCollected _asbp_orb_parent true)
    (Effects|SpawnEmitteratLocation "/Game/InfinityBladeEffects/Effects/FX_Ability/Defense/P_Shield_Spawn.P_Shield_Spawn" (Transformation|GetActorLocation OtherActor))))

(event Custom|CustomEvent
  (bind _returnvalue (UserInterface|CreateWidget "/Game/JimLastUpdated/FadeHUD.FadeHUD_C"))
  (UserInterface|Viewport|AddtoViewport _returnvalue 0)
  (Default|StartFadein _returnvalue))

(event EventBeginPlay
  (Transformation|SetWorldLocation (Variables|Default|GetDefaultSceneRoot) "0.000000, 0,900.000000" false false))

(event EventTick
  (params (DeltaSeconds :type Float%20%28single-precision%29))
  (bind _mc_right (Variables|Default|GetMC_right))
  (bind _mc_left (Variables|Default|GetMC_left))
  (Transformation|SetWorldLocationAndRotation (Variables|Default|GetGunL) (Transformation|GetWorldLocation _mc_left) (Transformation|GetWorldRotation _mc_left) false false)
  (Transformation|SetWorldLocationAndRotation (Variables|Default|GetGunR) (Transformation|GetWorldLocation _mc_right) (Transformation|GetWorldRotation _mc_right) false false))

(event Input|KeyboardEvents|W
  (params (Key :type Key%20Structure :default "AnyKey"))
  (bind _manus_handv2_left (Variables|Default|GetManus_Handv2_Left))
  (bind _returnvalue (Transformation|GetRelativeTransform _manus_handv2_left))
  (:Pressed
    (Components|MoveComponentTo (Variables|Default|GetManus_Handv2_Left) (.location _returnvalue) (Math|Rotator|MakeRotator (.roll (.rotation _returnvalue)) (.pitch (.rotation _returnvalue)) (+ (.yaw (.rotation _returnvalue)) 2e+01)) true true 0.2)))

(event Input|KeyboardEvents|MotionControllerLeftTrigger
  (params (Key :type Key%20Structure :default "AnyKey"))
  (bind _mc_left (Variables|Default|GetMC_left))
  (:Pressed
    (Variables|Default|SetIsPressedL true))
  (:Released
    (Variables|Default|SetIsPressedL false)
    (Utilities|MultiFireLoop (Variables|Default|GetOrbsL) (Transformation|GetWorldLocation _mc_left) (Math|Vector|GetForwardVector _mc_left) :!label _label
      (:Loop%20Body
        (Utilities|Empty
          (:Output
            (goto _label)))))))

(event Input|KeyboardEvents|S
  (params (Key :type Key%20Structure :default "AnyKey"))
  (bind _manus_handv2_right (Variables|Default|GetManus_Handv2_Right))
  (bind _returnvalue (Transformation|GetRelativeTransform _manus_handv2_right))
  (:Pressed
    (Components|MoveComponentTo (Variables|Default|GetManus_Handv2_Right) (.location _returnvalue) (Math|Rotator|MakeRotator (.roll (.rotation _returnvalue)) (.pitch (.rotation _returnvalue)) (+ (.yaw (.rotation _returnvalue)) 2e+01)) true true 0.2)))

(event Input|KeyboardEvents|MotionControllerRightTrigger
  (params (Key :type Key%20Structure :default "AnyKey"))
  (bind _mc_right (Variables|Default|GetMC_right))
  (:Pressed
    (Variables|Default|SetIsPressedR true))
  (:Released
    (Variables|Default|SetIsPressedR false)
    (Utilities|MultiFireLoop (Variables|Default|GetOrbsR) (Transformation|GetWorldLocation _mc_right) (Math|Vector|GetForwardVector _mc_right) :!label _label
      (:Loop%20Body
        (Utilities|Empty
          (:Output
            (goto _label)))))))

(fn ConstructionScript)

(fn UpdateIndexL
  (params (Index :type Integer))
  (Math|Integer|CompareInt (Variables|Default|GetIndexL) Index
    (:>
      _)
    (:<
      _))
  (Variables|Default|SetIndexL Index)
  (CallFunction|UpdateHandColors)
  (Utilities|IsValid (Variables|Default|GetSelectedOrbL)
    (:Is%20Valid
      (Default|StopMoving (Variables|Default|GetSelectedOrbL))
      (Variables|Default|SetSelectedOrbL 0))))

(fn UpdateIndexR
  (params (Index :type Integer))
  (Math|Integer|CompareInt Index (Variables|Default|GetIndexR)
    (:>
      _)
    (:<
      _))
  (Variables|Default|SetIndexR Index)
  (CallFunction|UpdateHandColors)
  (Utilities|IsValid (Variables|Default|GetSelectedOrbR)
    (:Is%20Valid
      (Default|StopMoving (Variables|Default|GetSelectedOrbR))
      (Variables|Default|SetSelectedOrbR 0))))

(fn UpdateHandColors
  (bind _rightsound (Variables|Default|GetRightSound))
  (bind _leftsound (Variables|Default|GetLeftSound))
  (bind _manus_handv2_left (Variables|Default|GetManus_Handv2_Left))
  (bind _manus_handv2_right (Variables|Default|GetManus_Handv2_Right))
  (switch int (Variables|Default|GetIndexL)
    (:Default
      (Rendering|Material|SetMaterial _manus_handv2_left 0 "/Game/FBX/CentralePlatform/pasted__glow.pasted__glow")
      (Audio|Components|Audio|Stop _leftsound))
    (:0
      (Rendering|Material|SetMaterial _manus_handv2_left 0 "/Game/Materials/Green.Green")
      (Audio|Components|Audio|SetSound _leftsound "/Game/Sounds/Sounds/Enversed_water_Cue.Enversed_water_Cue")
      (Audio|Components|Audio|Play _leftsound 0.0 :!label _label))
    (:1
      (Rendering|Material|SetMaterial _manus_handv2_left 0 "/Game/ManusModel/Manus_Material.Manus_Material")
      (Audio|Components|Audio|SetSound _leftsound "/Game/Sounds/Sounds/Enversed_fire_Cue.Enversed_fire_Cue")
      (goto _label))
    (:2
      (Rendering|Material|SetMaterial _manus_handv2_left 0 "/Game/Materials/Green.Green")
      (Audio|Components|Audio|SetSound _leftsound "/Game/Sounds/Sounds/Enversed_electricity_Cue.Enversed_electricity_Cue")
      (goto _label)))
  (switch int (Variables|Default|GetIndexR)
    (:Default
      (Rendering|Material|SetMaterial _manus_handv2_right 0 0)
      (Audio|Components|Audio|Stop _rightsound))
    (:0
      (Rendering|Material|SetMaterial _manus_handv2_right 0 "/Game/ManusModel/Dark_Gray.Dark_Gray")
      (Audio|Components|Audio|SetSound _rightsound "/Game/Sounds/Sounds/Enversed_water_Cue.Enversed_water_Cue")
      (Audio|Components|Audio|Play _rightsound 0.0 :!label _label_2))
    (:1
      (Rendering|Material|SetMaterial _manus_handv2_right 0 "/Game/ManusModel/Manus_Material.Manus_Material")
      (Audio|Components|Audio|SetSound _rightsound "/Game/Sounds/Sounds/Enversed_fire_Cue.Enversed_fire_Cue")
      (goto _label_2))
    (:2
      (Rendering|Material|SetMaterial _manus_handv2_right 0 "/Game/Materials/Green.Green")
      (Audio|Components|Audio|SetSound _rightsound "/Game/Sounds/Sounds/Enversed_electricity_Cue.Enversed_electricity_Cue")
      (goto _label_2))))