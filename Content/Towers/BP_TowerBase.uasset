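; Base tower actor whose static mesh height tracks an elemental meter in the GM_OrbCollection game mode.
; BeginPlay caches the game mode and starting location as the full-meter height.
; Each Tick, OrbIndex selects the Fire, Water or Lightning meter, which maps to a downward offset of up to MaxZDisplacement.
; Rises ease in through a per-frame, frame-rate-dependent Lerp, while drops snap immediately.
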(event EventBeginPlay
  (bind _staticmesh (Variables|Default|GetStaticMesh))
  (bind _returnvalue (Transformation|GetWorldLocation _staticmesh))
  (Variables|Default|SetInitialLocation _returnvalue)
  (Variables|Default|SetInitialLocationZ (.Z (Math|Vector|BreakVector _returnvalue)))
  (bind _asgm_orb_collection (Utilities|Casting|CastToGM_OrbCollection (Game|GetGameMode)))
  (Variables|Default|SetGameMode _asgm_orb_collection))

(event EventTick
  (params (DeltaSeconds :type Float%20%28single-precision%29))
  (bind _gamemode (Variables|Default|GetGameMode))
  (bind _maxzdisplacement (Variables|Default|GetMaxZDisplacement))
  (bind _initiallocation (Variables|Default|GetInitialLocation))
  (bind _initiallocationz (Variables|Default|GetInitialLocationZ))
  (bind _initiallocation_2 (Variables|Default|GetInitialLocation))
  (bind _gamemode_2 (Variables|Default|GetGameMode))
  (bind _maxzdisplacement_2 (Variables|Default|GetMaxZDisplacement))
  (bind _initiallocation_3 (Variables|Default|GetInitialLocation))
  (bind _initiallocationz_2 (Variables|Default|GetInitialLocationZ))
  (bind _maxzdisplacement_3 (Variables|Default|GetMaxZDisplacement))
  (bind _initiallocation_4 (Variables|Default|GetInitialLocation))
  (bind _gamemode_3 (Variables|Default|GetGameMode))
  (bind _maxzdisplacement_4 (Variables|Default|GetMaxZDisplacement))
  (bind _initiallocation_5 (Variables|Default|GetInitialLocation))
  (bind _initiallocationz_3 (Variables|Default|GetInitialLocationZ))
  (bind _maxzdisplacement_5 (Variables|Default|GetMaxZDisplacement))
  (bind _initiallocation_6 (Variables|Default|GetInitialLocation))
  (bind _maxzdisplacement_6 (Variables|Default|GetMaxZDisplacement))
  (bind _lightningmeter (Variables|/Game/Orbs/GM_OrbCollection.GM_OrbCollection_C|GetLightningMeter _gamemode_2))
  (bind _firemeter (Variables|/Game/Orbs/GM_OrbCollection.GM_OrbCollection_C|GetFireMeter _gamemode_3))
  (bind _watermeter (Variables|/Game/Orbs/GM_OrbCollection.GM_OrbCollection_C|GetWaterMeter _gamemode))
  (bind _returnvalue (/ _lightningmeter 1e+02))
  (bind _returnvalue_2 (/ _firemeter 1e+02))
  (bind _returnvalue_3 (/ _watermeter 1e+02))
  (bind _returnvalue_4 (* _returnvalue_3 _maxzdisplacement))
  (bind _returnvalue_5 (* _returnvalue _maxzdisplacement_2))
  (bind _returnvalue_6 (* _returnvalue_2 _maxzdisplacement_4))
  (bind _returnvalue_7 (- _maxzdisplacement_3 _returnvalue_5))
  (bind _returnvalue_8 (- _maxzdisplacement_5 _returnvalue_6))
  (bind _returnvalue_9 (- _maxzdisplacement_6 _returnvalue_4))
  (bind _returnvalue_10 (- _initiallocationz_2 _returnvalue_7))
  (bind _returnvalue_11 (- _initiallocationz_3 _returnvalue_8))
  (bind _returnvalue_12 (- _initiallocationz _returnvalue_9))
  (Variables|Default|SetLastLocationZ (.Z (Math|Vector|BreakVector (Transformation|GetWorldLocation (Variables|Default|GetStaticMesh)))))
  (switch int (Variables|Default|GetOrbIndex)
    (:0
      (if (> _returnvalue_11 (Variables|Default|GetLastLocationZ))
        (bind _output_get (Variables|Default|SetNewLocationZ (Math|Float|Lerp _returnvalue_11 (Variables|Default|GetLastLocationZ) 0.995)))
        (Transformation|SetWorldLocation (Variables|Default|GetStaticMesh) (Math|Vector|MakeVector (.x _initiallocation_5) (.y _initiallocation_5) _output_get) false false)
        (else
          (Transformation|SetWorldLocation (Variables|Default|GetStaticMesh) (Math|Vector|MakeVector (.x _initiallocation_6) (.y _initiallocation_6) _returnvalue_11) false false))))
    (:1
      (if (> _returnvalue_12 (Variables|Default|GetLastLocationZ))
        (bind _output_get_2 (Variables|Default|SetNewLocationZ (Math|Float|Lerp _returnvalue_12 (Variables|Default|GetLastLocationZ) 0.995)))
        (Transformation|SetWorldLocation (Variables|Default|GetStaticMesh) (Math|Vector|MakeVector (.x _initiallocation_2) (.y _initiallocation_2) _output_get_2) false false)
        (else
          (Transformation|SetWorldLocation (Variables|Default|GetStaticMesh) (Math|Vector|MakeVector (.x _initiallocation) (.y _initiallocation) _returnvalue_12) false false))))
    (:2
      (if (> _returnvalue_10 (Variables|Default|GetLastLocationZ))
        (bind _output_get_3 (Variables|Default|SetNewLocationZ (Math|Float|Lerp _returnvalue_10 (Variables|Default|GetLastLocationZ) 0.995)))
        (Transformation|SetWorldLocation (Variables|Default|GetStaticMesh) (Math|Vector|MakeVector (.x _initiallocation_3) (.y _initiallocation_3) _output_get_3) false false)
        (else
          (Transformation|SetWorldLocation (Variables|Default|GetStaticMesh) (Math|Vector|MakeVector (.x _initiallocation_4) (.y _initiallocation_4) _returnvalue_10) false false))))))

(fn ConstructionScript)