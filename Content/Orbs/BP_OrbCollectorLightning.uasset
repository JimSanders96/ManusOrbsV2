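; BP_OrbCollectorLightning is an orb collector that turns overlapping orbs of its own type into orb meter progress.
; It caches GM_OrbCollection on BeginPlay and, on overlap, accepts only BP_OrbParent actors whose OrbIndex matches its own.
; CollectOrb passes the orb's ScoreValue to the game mode's FillOrbMeter, then flags and destroys the orb, or prints a debug string if the game mode is invalid.
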(event Collision|EventActorBeginOverlap
  (params (OtherActor :type Actor%20Object%20Reference))
  (bind _asbp_orb_parent (Utilities|Casting|CastToBP_OrbParent OtherActor))
  (if (== (Variables|/Game/Orbs/BP_OrbParent.BP_OrbParent_C|GetOrbIndex _asbp_orb_parent) (Variables|Default|GetOrbIndex))
    (CallFunction|CollectOrb _asbp_orb_parent)))

(event EventBeginPlay
  (bind _asgm_orb_collection (Utilities|Casting|CastToGM_OrbCollection (Game|GetGameMode)))
  (Variables|Default|SetGameMode _asgm_orb_collection))

(fn ConstructionScript)

(fn CollectOrb
  (params (Orb :type BP%20Orb%20Parent%20Object%20Reference))
  (bind _gamemode (Variables|Default|GetGameMode))
  (if (Utilities|IsValid _gamemode)
    (Default|FillOrbMeter _gamemode (Variables|Default|GetOrbIndex) (Variables|/Game/Orbs/BP_OrbParent.BP_OrbParent_C|GetScoreValue Orb))
    (Variables|/Game/Orbs/BP_OrbParent.BP_OrbParent_C|SetIsBeingDestroyed Orb true)
    (Actor|DestroyActor Orb)
    (else
      (Development|PrintString "Kutzooi"))))