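; Game mode for an orb collection game, tracking a countdown timer, score and Water, Fire and Lightning meters.
; Tick counts down and ramps the drain rate until game over.
; External callers fill, reset or drain meters, with fills also adding to score.
; Drain calls trigger the game-over check, which looks only at the timer, not meter levels, and shows the score widget on expiry.
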(event EventBeginPlay)

(event EventTick
  (params (DeltaSeconds :type Float%20%28single-precision%29))
  (Variables|Default|SetTimer (- (Variables|Default|GetTimer) DeltaSeconds))
  (if (not (Variables|Default|GetGameOver))
    (CallFunction|IncreaseDrainage DeltaSeconds)))

(fn ConstructionScript)

(fn DrainOrbMetersPerSecond
  (params (DeltaSeconds :type Float%20%28single-precision%29) (OrbIndex :type Integer))
  (bind _meterdrainagepersecond (Variables|Default|GetMeterDrainagePerSecond))
  (bind _returnvalue (* DeltaSeconds _meterdrainagepersecond))
  (switch int OrbIndex
    (:0
      (Variables|Default|SetWaterMeter (- (Variables|Default|GetWaterMeter) _returnvalue)))
    (:1
      (Variables|Default|SetFireMeter (- (Variables|Default|GetFireMeter) _returnvalue)))
    (:2
      (Variables|Default|SetLightningMeter (- (Variables|Default|GetLightningMeter) _returnvalue))))
  ;[1 1 1] Debug
  (Development|PrintString (Utilities|String|ToString(Float) 0.0) true true "(R=0.000000,G=0.660000,B=1.000000,A=1.000000)" 0.0)
  (CallFunction|CheckGameOver))

(fn CheckGameOver
  (if (<= (Variables|Default|GetTimer) 0.0)
    (Variables|Default|SetGameOver true)
    (bind _returnvalue (UserInterface|CreateWidget "/Game/JimLastUpdated/ScoreHUD.ScoreHUD_C" (Game|GetPlayerController 0)))
    (Default|SetScoreText _returnvalue (Variables|Default|GetScore))
    (UserInterface|Viewport|AddtoViewport _returnvalue 0)))

(fn FillOrbMeter
  (params (OrbIndex :type Integer) (Value :type Float%20%28single-precision%29))
  (switch int OrbIndex
    (:0
      (Variables|Default|SetWaterMeter (Math|Float|Clamp(Float) (+ (Variables|Default|GetWaterMeter) Value) 0.0 1e+02)))
    (:1
      (Variables|Default|SetFireMeter (Math|Float|Clamp(Float) (+ (Variables|Default|GetFireMeter) Value) 0.0 1e+02)))
    (:2
      (Variables|Default|SetLightningMeter (Math|Float|Clamp(Float) (+ (Variables|Default|GetLightningMeter) Value) 0.0 1e+02))))
  (bind _output_get (Variables|Default|SetScore (+ (Variables|Default|GetScore) (Math|Float|Truncate Value))))
  (Development|PrintString (Utilities|String|Append "Score: " (Utilities|String|ToString(Integer) _output_get))))

(fn DrainOrbMetersInstantly
  (params (InstantDrainage :type Float%20%28single-precision%29))
  (Variables|Default|SetFireMeter (- (Variables|Default|GetFireMeter) InstantDrainage))
  (Variables|Default|SetWaterMeter (- (Variables|Default|GetWaterMeter) InstantDrainage))
  (Variables|Default|SetLightningMeter (- (Variables|Default|GetLightningMeter) InstantDrainage))
  ;[1 1 1] Debug
  (Development|PrintString (Utilities|String|Append "Fire: " (Utilities|String|ToString(Float) 0.0)) true true "(R=0.000000,G=0.660000,B=1.000000,A=1.000000)" 0.0)
  ;[1 1 1] Debug
  (Development|PrintString (Utilities|String|Append "Water: " (Utilities|String|ToString(Float) 0.0)) true true "(R=0.000000,G=0.660000,B=1.000000,A=1.000000)" 0.0)
  ;[1 1 1] Debug
  (Development|PrintString (Utilities|String|Append "Lightning: " (Utilities|String|ToString(Float) 0.0)) true true "(R=0.000000,G=0.660000,B=1.000000,A=1.000000)" 0.0)
  (CallFunction|CheckGameOver))

(fn IncreaseDrainage
  (params (DeltaSeconds :type Float%20%28single-precision%29))
  (Variables|Default|SetMeterDrainagePerSecond (+ (Variables|Default|GetMeterDrainagePerSecond) (* DeltaSeconds (Variables|Default|GetDrainageIncrementPerSecond)))))

(fn ResetMeters
  (Variables|Default|SetFireMeter 1e+02)
  (Variables|Default|SetWaterMeter 1e+02)
  (Variables|Default|SetLightningMeter 1e+02))