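; BP_OrbCollector is an actor that collects orbs it overlaps and reports them to the game mode's orb meter.
; On overlap with a BP_OrbParent, CollectOrb passes the orb's index and score value to FillOrbMeter, then destroys the orb.
; BeginPlay casts the game mode to GM_OrbCollection but sets the GameMode variable to None, so the cast result is never stored for that call.
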(event Collision|EventActorBeginOverlap
  (params (OtherActor :type Actor%20Object%20Reference))
  (bind _asbp_orb_parent (Utilities|Casting|CastToBP_OrbParent OtherActor))
  (CallFunction|CollectOrb _asbp_orb_parent))

(event EventBeginPlay
  (Utilities|Casting|CastToGM_OrbCollection (Game|GetGameMode))
  (Variables|Default|SetGameMode 0))

(fn ConstructionScript)

(fn CollectOrb
  (params (Orb :type BP%20Orb%20Parent%20Object%20Reference))
  (Default|FillOrbMeter (Variables|Default|GetGameMode) (Variables|/Game/Orbs/BP_OrbParent.BP_OrbParent_C|GetOrbIndex Orb) (Variables|/Game/Orbs/BP_OrbParent.BP_OrbParent_C|GetScoreValue Orb))
  (Actor|DestroyActor Orb))