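; BP_OrbParent is a parent orb actor that floats upward and can move toward a target.
; Each tick it rises unless pulled, collected or being destroyed, optionally destroying itself above a death height.
; It also either lerps its collision to the target when other movement is ignored, or applies distance-scaled force when flagged as moving.
; Overlapping another orb makes its collision ignore that orb when moving.
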(event Custom|MoveByForce
  ;[1 1 1] MoveByForce
  (bind _collision (CallFunction|GetCollision))
  (Utilities|IsValid _collision
    (:Is%20Valid
      (Physics|AddForce _collision (* (- (Transformation|GetWorldLocation (Variables|Default|GetTarget)) (Transformation|GetWorldLocation _collision)) (Variables|Default|GetForce)) "None" false))))

(event Custom|MoveByTranslation
  ;[1 1 1] MoveTowardsPosition
  (bind _collision (CallFunction|GetCollision))
  (bind _collision_2 (CallFunction|GetCollision))
  (Utilities|IsValid _collision_2
    (:Is%20Valid
      (Transformation|SetWorldLocation _collision_2 (Math|Vector|Lerp(Vector) (Transformation|GetWorldLocation _collision) (Transformation|GetWorldLocation (Variables|Default|GetTarget)) 0.1) false false))))

(event Collision|EventActorBeginOverlap
  (params (OtherActor :type Actor%20Object%20Reference))
  (bind _asbp_orb_parent (Utilities|Casting|CastToBP_OrbParent OtherActor))
  (Collision|IgnoreActorwhenMoving (Variables|Default|GetCollision) _asbp_orb_parent true))

(event EventTick
  (params (DeltaSeconds :type Float%20%28single-precision%29))
  (bind _collision (Variables|Default|GetCollision))
  (bind _returnvalue (Transformation|GetWorldLocation _collision))
  (bind (_x _y _z) (Math|Vector|BreakVector _returnvalue))
  ;[1 1 1] Function for moving the orb upwards
  (Utilities|FlowControl|Sequence
    (:then_0
      (if (not (Variables|Default|GetIsBeingPulled))
        (if (not (Variables|Default|GetIsCollected))
          (if (not (Variables|Default|GetIsBeingDestroyed))
            (if (and (> _z (Variables|Default|GetDeathHeight)) (Variables|Default|GetDestroyOnHeight))
              (Actor|DestroyActor)
              (else
                (Transformation|SetWorldLocation _collision (Math|Vector|MakeVector _x _y (+ _z (Variables|Default|GetFloatSpeed))) false false)))))))
    (:then_1
      ;[1 1 1] Decide what movement should be used
      (if (Variables|Default|GetIgnoreOtherMovement)
        (CallFunction|MovebyTranslation)
        (elif (Variables|Default|GetIsMoving)
          (CallFunction|MovebyForce))))))

(event EventBeginPlay)

(fn ConstructionScript)

(fn GetCollision
  (return (Variables|Default|GetCollision)))