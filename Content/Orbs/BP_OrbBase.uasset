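; BP_OrbBase is a base orb actor that shrinks over time and carries a score value tied to its size.
; On Tick, unless the orb is being pulled, it scales its mesh down by a shrink speed adjusted for frame time.
; The score is recalculated from the length of the new scale vector, and the orb destroys itself once that length would fall below a small threshold.
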(event EventTick
  (params (DeltaSeconds :type Float%20%28single-precision%29))
  (bind _orbmesh (Variables|Default|GetOrbMesh))
  (bind _shrinkspeed_0 (Variables|Default|GetShrinkSpeed_0))
  (bind _returnvalue (Transformation|GetWorldScale _orbmesh))
  (bind _returnvalue_2 (* _shrinkspeed_0 DeltaSeconds))
  (bind _returnvalue_3 (- 1.0 _returnvalue_2))
  (bind _returnvalue_4 (* _returnvalue _returnvalue_3))
  ;[1 1 1] Function for shrinking the orb
  (if (not (Variables|Default|GetIsBeingPulled_0))
    (if (< (Math|Vector|VectorLength _returnvalue_4) 0.5)
      (Actor|DestroyActor)
      (else
        (Transformation|SetWorldScale3D _orbmesh _returnvalue_4)
        (Variables|Default|SetScoreValue_0 (* (Math|Vector|VectorLength (Transformation|GetWorldScale (Variables|Default|GetOrbMesh))) 1e+01))))))

(fn ConstructionScript)